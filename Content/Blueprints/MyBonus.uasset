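; MyBonus is a bonus actor that awards score to whoever damages it.
; On any damage, the authority casts the instigator's player state to MyPlayerState, increments its score and destroys the actor.
; The construction script adds a random number of static mesh components, each placed at a random unit vector scaled by zero, so with no offset.
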(event `self.ReceiveAnyDamage`
  (params (Damage :type "Float (single-precision)") (DamageType :type "DamageType Object Reference") (InstigatedBy :type "Controller Object Reference") (DamageCauser :type "Actor Object Reference"))
  (`/Engine/EditorBlueprintResources/ActorMacros.Switch Has Authority`
    (:`Authority`
      (bind _asmy_player_state (cast `/Game/Blueprints/MyPlayerState` (`Controller.PlayerState` InstigatedBy)))
      (`/Game/Blueprints/MyPlayerState.IncrementScore` _asmy_player_state)
      (`self.K2_DestroyActor` self))))

(fn `UserConstructionScript`
  (for _ (range 1 (+ (`self.random`) 1))
    (`AddComponent|NODE_AddStaticMeshComponent-0` :`RelativeTransform` (`KismetMathLibrary.Conv_VectorToTransform` (* (`KismetMathLibrary.RandomUnitVector`) 0.0)))))